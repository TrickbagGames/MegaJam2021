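; BP_Conveyor is a level conveyor that carries characters along while its gears spin.
; On BeginPlay it starts a looping 0.01-second timer that drives GearUpdate, in place of Tick.
; Each update rotates seven gear components and nudges every BP_Base_Character overlapping the Box along the Arrow's forward vector, with sweep.
; Movement is a fixed step per timer call, and the ConveyorStart event is empty.
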(event `self.ReceiveBeginPlay`
  (`self.Start Gear Rotation`))

(event `Gear Update`
  (`SceneComponent.K2_AddLocalRotation` (`self.Gear01`) (`KismetMathLibrary.MakeRotator` 0.0 1.0) false false)
  (`SceneComponent.K2_AddLocalRotation` (`self.Gear02`) (`KismetMathLibrary.MakeRotator` 0.0 1.0) false false)
  (`SceneComponent.K2_AddLocalRotation` (`self.Gear03`) (`KismetMathLibrary.MakeRotator` 0.0 1.0) false false)
  (`SceneComponent.K2_AddLocalRotation` (`self.Gear04`) (`KismetMathLibrary.MakeRotator` 0.0 1.0) false false)
  (`SceneComponent.K2_AddLocalRotation` (`self.Gear05`) (`KismetMathLibrary.MakeRotator` 0.0 1.0) false false)
  (`SceneComponent.K2_AddLocalRotation` (`self.Gear06`) (`KismetMathLibrary.MakeRotator` 0.0 1.0) false false)
  (`SceneComponent.K2_AddLocalRotation` (`self.Gear07`) (`KismetMathLibrary.MakeRotator` 0.0 1.0) false false)
  (for _array_element (`PrimitiveComponent.GetOverlappingActors` (`self.Box`) "/Script/Engine.Actor")
    (bind _asbp_base_character (cast `/Game/Game/Classes/Character/BP_Base_Character` _array_element))
    (`self.K2_AddActorWorldOffset` _asbp_base_character (* (`SceneComponent.GetForwardVector` (`self.Arrow`)) 1.0) true false)))

(event `Start Gear Rotation`
  (`KismetSystemLibrary.K2_SetTimerDelegate` (delegate `Gear Update`) 0.01 true))

(event `Conveyor Start`)

(fn `UserConstructionScript`)