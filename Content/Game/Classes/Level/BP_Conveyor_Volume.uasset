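; Conveyor volume that pushes BP_Base_Character actors inside its box along the arrow's forward direction.
; A character entering the box starts a fast looping timer that moves each overlapping character by a small swept world offset.
; Any end overlap clears the timer, with no check on the actor leaving or on characters still inside.
; The construction script sizes the box from the BoxExtent variable.
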(event `Conveyor Update`
  (for _array_element (`PrimitiveComponent.GetOverlappingActors` (`self.Box`) "/Game/Game/Classes/Character/BP_Base_Character.BP_Base_Character_C")
    (`self.K2_AddActorWorldOffset` _array_element (* (`SceneComponent.GetForwardVector` (`self.Arrow`)) 1.0) true false)))

(event `Conveyor Start`
  (bind _returnvalue (`KismetSystemLibrary.K2_SetTimerDelegate` (delegate `Conveyor Update`) 0.01 true))
  (set `self.ConveyorTimer` _returnvalue))

(event `Stop Conveyor`
  (`KismetSystemLibrary.K2_ClearAndInvalidateTimerHandle` (`self.ConveyorTimer`)))

(event `self.Box.OnComponentBeginOverlap`
  (params (OverlappedComponent :type "PrimitiveComponent Object Reference") (OtherActor :type "Actor Object Reference") (OtherComp :type "PrimitiveComponent Object Reference") (OtherBodyIndex :type Integer) (bFromSweep :type Boolean) (SweepResult :type "HitResult Structure (by ref)"))
  (cast `/Game/Game/Classes/Character/BP_Base_Character` OtherActor)
  (`self.Conveyor Start`))

(event `self.Box.OnComponentEndOverlap`
  (params (OverlappedComponent :type "PrimitiveComponent Object Reference") (OtherActor :type "Actor Object Reference") (OtherComp :type "PrimitiveComponent Object Reference") (OtherBodyIndex :type Integer))
  (`self.Stop Conveyor`))

(fn `UserConstructionScript`
  (`BoxComponent.SetBoxExtent` (`self.Box`) (`self.BoxExtent`) true))