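; BP_Laser_Test is a test laser actor that aims a stretched mesh beam at a target actor and disintegrates it.
; Each tick, it smoothly rotates the mesh toward ActorTarget and scales its length by the distance to that target.
; A DoOnce triggers Disintegrate a single time if the target is a BP_Base_Character.
; Without a valid target, the beam mesh is hidden and never made visible again here.
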(event `self.ReceiveTick`
  (params (DeltaSeconds :type "Float (single-precision)"))
  (bind _actor_target (`self.Actor Target`))
  (bind _staticmesh (`self.StaticMesh`))
  (bind _staticmesh_2 (`self.StaticMesh`))
  (bind _returnvalue (`self.K2_GetActorLocation` _actor_target))
  (`/Engine/EditorBlueprintResources/StandardMacros.IsValid` _actor_target
    (:`Is Valid`
      (`SceneComponent.K2_SetWorldRotation` _staticmesh (`KismetMathLibrary.RInterpTo` (`SceneComponent.K2_GetComponentRotation` _staticmesh_2) (`KismetMathLibrary.FindLookAtRotation` (`SceneComponent.K2_GetComponentLocation` _staticmesh_2) _returnvalue) DeltaSeconds 50.0) false false)
      (`SceneComponent.SetWorldScale3D` _staticmesh (`KismetMathLibrary.MakeVector` (* (/ (`self.GetDistanceTo` _actor_target) 10.0) 1.0) 0.5 0.5))
      (`/Engine/EditorBlueprintResources/StandardMacros.DoOnce` false
        (:`Completed`
          (bind _asbp_base_character (cast `/Game/Game/Classes/Character/BP_Base_Character` _actor_target))
          (`/Game/Game/Classes/Character/BP_Base_Character.Disintegrate` _asbp_base_character _returnvalue))))
    (:`Is Not Valid`
      (`SceneComponent.SetVisibility` (`self.StaticMesh`) false false))))

(fn `UserConstructionScript`)