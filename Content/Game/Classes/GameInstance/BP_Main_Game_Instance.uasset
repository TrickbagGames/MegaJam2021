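; BP_Main_Game_Instance is the game instance, holding FileScanQueryList, an ordered list of files that by its name are awaiting scanning.
; Events append a file to the list or remove one at the index returned by GetQueryPosition.
; AdjustQueryPosition moves a file to a given slot by removing it and reinserting it there.
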(event `Add File to List`
  (params (File :type "/Game/Game/Classes/Character/BP_Base_Character Object Reference"))
  (`KismetArrayLibrary.Array_Add` (`self.FileScanQueryList`) File))

(event `Remove File Query`
  (params (FileRef :type "/Game/Game/Classes/Character/BP_Base_Character Object Reference"))
  (bind _position (`self.Get Query Position` FileRef))
  (`KismetArrayLibrary.Array_Remove` (`self.FileScanQueryList`) _position))

(fn `Adjust Query Position`
  (params (Slot :type Integer) (`File Ref` :type "/Game/Game/Classes/Character/BP_Base_Character Object Reference"))
  (locals (FileRefLocal :type "/Game/Game/Classes/Character/BP_Base_Character Object Reference"))
  (bind _filescanquerylist (`self.FileScanQueryList`))
  (`KismetArrayLibrary.Array_Remove` _filescanquerylist (`KismetArrayLibrary.Array_Find` _filescanquerylist `File Ref`))
  (`KismetArrayLibrary.Array_Insert` _filescanquerylist `File Ref` Slot))

(fn `Get Query Position`
  (params (`File Ref` :type "/Game/Game/Classes/Character/BP_Base_Character Object Reference"))
  (returns (Position :type Integer))
  (return (`KismetArrayLibrary.Array_Find` (`self.FileScanQueryList`) `File Ref`)))