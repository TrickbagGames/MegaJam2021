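; Base character Blueprint that moves along a fixed world X axis and can carry a randomized file identity.
; The forward/backward input axis feeds inverted movement input; Tick is empty.
; When RandomFile is set, the construction script picks a random row from Table_Files and, independently, one of ten file types.
; It builds the FileName text by appending the type's enum string to the row's name.
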(event `self.ReceiveTick`
  (params (DeltaSeconds :type "Float (single-precision)")))

(event `InputAxis|Move Forward/Backward`
  (params (AxisValue :type "Float (single-precision)"))
  (`self.AddMovementInput` (1.0 0.0 0.0) (* AxisValue -1.0)))

(fn `UserConstructionScript`
  (if (`self.bRandomFile?`)
    (bind _outrownames (`DataTableFunctionLibrary.GetDataTableRowNames` "/Game/Game/Data/Table/Table_Files.Table_Files"))
    (bind _returnvalue (`|GetDataTableRow` "/Game/Game/Data/Table/Table_Files.Table_Files" (`|GetArrayItem` _outrownames (`KismetMathLibrary.RandomIntegerInRange` 0 (- (`KismetArrayLibrary.Array_Length` _outrownames) 1))))
      (:`then`
        (bind _output_get (set `self.FileType` (select `int` (`KismetMathLibrary.RandomIntegerInRange` 0 9) :`0` "NewEnumerator0" :`1` "NewEnumerator1" :`2` "NewEnumerator2" :`3` "NewEnumerator3" :`4` "NewEnumerator4" :`5` "NewEnumerator5" :`6` "NewEnumerator6" :`7` "NewEnumerator7" :`8` "NewEnumerator8" :`9` "NewEnumerator9" :!type "/Game/Game/Data/Enum/Enum_FileType Enum")))
        (set `self.FileName` (`KismetTextLibrary.Conv_StringToText` (`KismetStringLibrary.Concat_StrStr` (`.FileName_6_0C4F6F5944D4213C968038855A24C3FC` (break `/Game/Game/Data/Struct/Struct_File` _returnvalue)) (`|GetEnumeratorNameAsString` _output_get))))))))